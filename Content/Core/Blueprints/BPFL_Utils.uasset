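; Blueprint function library of utilities, with one function, ChangeValueAtRate, that steps a float toward a target at a constant rate.
; The step is the absolute per-second rate times delta time, applied in the direction of the target, so the sign of the rate is irrelevant.
; When the remaining distance is within one step, it returns the target exactly to avoid overshoot.
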(fn `ChangeValueAtRate`
  (params (From :type "Float (double-precision)") (To :type "Float (double-precision)") (DeltaPerSecond :type "Float (double-precision)") (DeltaT :type "Float (double-precision)"))
  (returns (Value :type "Float (double-precision)"))
  (locals (Result :type "Float (double-precision)"))
  (bind _returnvalue (- To From))
  (bind _returnvalue_2 (* (`KismetMathLibrary.Abs` DeltaPerSecond) DeltaT))
  (if (<= (`KismetMathLibrary.Abs` _returnvalue) _returnvalue_2)
    (set `local.Result` To)
    (else
      (set `local.Result` (+ From (* _returnvalue_2 (`KismetMathLibrary.SignOfFloat` _returnvalue))))))
  (return (`local.Result`)))