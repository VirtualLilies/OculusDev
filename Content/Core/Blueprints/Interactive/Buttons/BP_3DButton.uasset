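; BP_3DButton is a VR 3D button that fires a Trigger event with its Value when pressed by a finger collider or laser.
; Tick projects the fingertip into border space to slide the fill, scaling glow and haptics until full press.
; Triggering plays a sound and glow timeline, with a short ignore window against retriggers.
; The construction script configures size meshes, icon, caption and colors through material parameters.
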(event `self.ReceiveBeginPlay`
  (add `/Game/Core/Blueprints/UI/LaserInteractionComponent.IndexAction` (`self.LaserInteractionComponent`) (delegate `LaserCall`))
  (set `self.DefaultDistance` (.y (`SceneComponent.RelativeLocation` (`self.BtnFill`)))))

(event `LaserCall`
  (params (instigator :type "/Game/Core/Blueprints/Hand/BP_Hand Object Reference"))
  ;[1 1 1] Called by laser
  (if (not (> (`self.IgnoreTime`) 0.0))
    (`self.Triggered`)
    (`PlayerController.PlayHapticEffect` (`GameplayStatics.GetPlayerController` 0) "/Game/Core/Haptics/ButtonClick.ButtonClick" (`/Game/Core/Blueprints/Hand/BP_Hand.HandType` instigator) 1.0 false)))

(event `self.ReceiveActorBeginOverlap`
  (params (OtherActor :type "Actor Object Reference"))
  ;[1 1 1] Add new collider
  (if (not (> (`self.IgnoreTime`) 0.0))
    (bind _asbp_finger_collider (cast `/Game/Core/Blueprints/Hand/BP_FingerCollider` OtherActor))
    (`self.FocusGain`)
    (set `self.Overlapping Collider` _asbp_finger_collider)))

(event `self.ReceiveActorEndOverlap`
  (params (OtherActor :type "Actor Object Reference"))
  ;[1 1 1] Clear collider
  (if (== OtherActor (`self.Overlapping Collider`))
    (`self.FocusLost`)
    (`PlayerController.StopHapticEffect` (`GameplayStatics.GetPlayerController` 0) (`/Game/Core/Blueprints/Hand/BP_FingerCollider.Hand` (`self.Overlapping Collider`)))
    (set `self.Overlapping Collider` null)
    (`SceneComponent.K2_SetRelativeLocation` (`self.BtnFill`) (`KismetMathLibrary.MakeVector` 0.0 (`self.DefaultDistance`)) false false)
    (`MeshComponent.SetScalarParameterValueOnMaterials` (`self.BtnBorder`) "Intensity" 0.0)))

(event `self.ReceiveTick`
  (params (DeltaSeconds :type "Float (single-precision)"))
  (bind _defaultdistance (`self.DefaultDistance`))
  (bind _progress (`self.Progress`))
  (bind _btnfill (`self.BtnFill`))
  (bind _returnvalue (`KismetMathLibrary.FClamp` (.y (`KismetMathLibrary.InverseTransformLocation` (`SceneComponent.K2_GetComponentToWorld` (`self.BtnBorder`)) (`SceneComponent.K2_GetComponentLocation` (`/Game/Core/Blueprints/Hand/BP_FingerCollider.Sphere` (`self.Overlapping Collider`))))) 0.0 _defaultdistance))
  ;[1 1 1] Adjust ignore time
  (set `self.IgnoreTime` (`KismetMathLibrary.FMax` (- (`self.IgnoreTime`) DeltaSeconds)))
  (`/Engine/EditorBlueprintResources/StandardMacros.IsValid` (`self.Overlapping Collider`)
    (:`Is Valid`
      ;[1 1 1] Process activation related to index finger activity
      (`SceneComponent.K2_SetRelativeRotation` _btnfill (struct :`Pitch` 180.0) false false)
      (set `self.Progress` (- 1.0 (/ _returnvalue _defaultdistance)))
      (`SceneComponent.K2_SetRelativeLocation` _btnfill (`KismetMathLibrary.MakeVector` 0.0 _returnvalue) false false)
      (if (== (`self.Progress`) 1.0)
        (`PlayerController.PlayHapticEffect` (`GameplayStatics.GetPlayerController` 0) "/Game/Core/Haptics/ButtonClick.ButtonClick" (`/Game/Core/Blueprints/Hand/BP_FingerCollider.Hand` (`self.Overlapping Collider`)) 1.0 false)
        (set `self.Overlapping Collider` null)
        (`self.Triggered`)
        (else
          (`MeshComponent.SetScalarParameterValueOnMaterials` (`self.BtnBorder`) "Intensity" _progress)
          (`PlayerController.SetHapticsByValue` (`GameplayStatics.GetPlayerController` 0) 0.0 (/ _progress 2.0) (`/Game/Core/Blueprints/Hand/BP_FingerCollider.Hand` (`self.Overlapping Collider`))))))
    (:`Is Not Valid`
      ;[1 1 1] Focus by laser, but only if animation is not running
      (if (not (`self.AnimationRunning`))
        (`MeshComponent.SetScalarParameterValueOnMaterials` (`self.BtnBorder`) "Intensity" (`KismetMathLibrary.SelectFloat` 0.65 0.0 (`/Game/Core/Blueprints/UI/LaserInteractionComponent.HasFocus` (`self.LaserInteractionComponent`))))))))

(event `Triggered`
  ;[1 1 1] Called
  (`GameplayStatics.PlaySoundAtLocation` null (`self.K2_GetActorLocation`) (struct) 1.0 1.0 0.0 null null null)
  (`self.Trigger` (`self.Value`))
  (`/Engine/EditorBlueprintResources/StandardMacros.IsValid` self ; In some cases, button may become invalid after trigger - destroyed
    (:`Is Valid`
      (set `self.IgnoreTime` 0.35)
      (bind (_direction _intensity) (`Timeline|Timeline_0` :!via `PlayFromStart`)
        (:`Update`
          (`MeshComponent.SetScalarParameterValueOnMaterials` (`self.BtnBorder`) "Intensity" _intensity)
          (set `self.AnimationRunning` true))
        (:`Finished`
          (`SceneComponent.K2_SetRelativeLocation` (`self.BtnFill`) (`KismetMathLibrary.MakeVector` 0.0 (`self.DefaultDistance`)) false false)
          (set `self.AnimationRunning` false))))))

(fn `SetCaption`
  (params (Text :type Text))
  (bind _output_get (set `self.CaptionText` Text))
  (`TextRenderComponent.K2_SetText` (`self.Caption`) _output_get))

(fn `SetIcon`
  (params (Icon :type "Texture Object Reference"))
  (bind _output_get (set `self.Icon` Icon))
  (`MaterialInstanceDynamic.SetTextureParameterValue` (`self.IconMat`) "Icon" _output_get))

(fn `SetType`
  (params (Type :type Byte))
  (switch `|SwitchEnum` Type
    (:`NewEnumerator0`
      (`StaticMeshComponent.SetStaticMesh` (`self.BtnBorder`) "/Game/Core/Blueprints/Interactive/Buttons/SM_ButtonBorder.SM_ButtonBorder")
      (`StaticMeshComponent.SetStaticMesh` (`self.BtnFill`) "/Game/Core/Blueprints/Interactive/Buttons/SM_Button.SM_Button"))
    (:`NewEnumerator2`
      (`StaticMeshComponent.SetStaticMesh` (`self.BtnBorder`) "/Game/Core/Blueprints/Interactive/Buttons/SM_2x1ButtonBorder.SM_2x1ButtonBorder")
      (`StaticMeshComponent.SetStaticMesh` (`self.BtnFill`) "/Game/Core/Blueprints/Interactive/Buttons/SM_2x1Button.SM_2x1Button"))
    (:`NewEnumerator3`
      (`StaticMeshComponent.SetStaticMesh` (`self.BtnBorder`) "/Game/Core/Blueprints/Interactive/Buttons/SM_Btn4x1_Border.SM_Btn4x1_Border")
      (`StaticMeshComponent.SetStaticMesh` (`self.BtnFill`) "/Game/Core/Blueprints/Interactive/Buttons/SM_Btn4x1.SM_Btn4x1"))
    (:`NewEnumerator1`
      (`StaticMeshComponent.SetStaticMesh` (`self.BtnBorder`) "/Game/Core/Blueprints/Interactive/Buttons/SM_UIButtonWideBorder.SM_UIButtonWideBorder")
      (`StaticMeshComponent.SetStaticMesh` (`self.BtnFill`) "/Game/Core/Blueprints/Interactive/Buttons/SM_UIButtonWide.SM_UIButtonWide"))
    (:`NewEnumerator4`
      (`StaticMeshComponent.SetStaticMesh` (`self.BtnBorder`) "/Game/Core/Blueprints/Interactive/Buttons/SM_Btn2x2_Border.SM_Btn2x2_Border")
      (`StaticMeshComponent.SetStaticMesh` (`self.BtnFill`) "/Game/Core/Blueprints/Interactive/Buttons/SM_Btn2x2.SM_Btn2x2"))
    (:`NewEnumerator5`
      (`StaticMeshComponent.SetStaticMesh` (`self.BtnBorder`) "/Game/Core/Blueprints/Interactive/Buttons/SM_4x4_Border.SM_4x4_Border")
      (`StaticMeshComponent.SetStaticMesh` (`self.BtnFill`) "/Game/Core/Blueprints/Interactive/Buttons/SM_Btn4x4.SM_Btn4x4"))
    (:`NewEnumerator6`
      (`StaticMeshComponent.SetStaticMesh` (`self.BtnBorder`) "/Game/Core/Blueprints/Interactive/Buttons/SM_Btn6x6_Border.SM_Btn6x6_Border")
      (`StaticMeshComponent.SetStaticMesh` (`self.BtnFill`) "/Game/Core/Blueprints/Interactive/Buttons/SM_Btn6x6.SM_Btn6x6"))))

(fn `UserConstructionScript`
  (bind _returnvalue (`PrimitiveComponent.CreateDynamicMaterialInstance` (`self.BtnFill`) 0 "/Game/Core/Blueprints/Interactive/Buttons/M_ButtonFront.M_ButtonFront" "None"))
  (bind _output_get (set `self.IconMat` _returnvalue))
  (`MaterialInstanceDynamic.SetVectorParameterValue` _output_get "Color" (`self.InnerColor`))
  (`self.SetIcon` (`self.Icon`))
  (`self.SetType` (`self.Type`))
  (`self.SetCaption` (`self.CaptionText`))
  (`MeshComponent.SetVectorParameterValueOnMaterials` (`self.BtnBorder`) "Color" (`KismetMathLibrary.Conv_LinearColorToVector` (`self.OuterColor`))))