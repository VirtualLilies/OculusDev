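; Interactive slider actor that the player drags with a finger collider or a laser pointer to set a 0–1 Progress value.
; An overlapping finger on Tick, or an active BPCLaserInteract laser, supplies a local X position that becomes clamped Progress.
; Progress moves the knob, drives the track material with an edge-margin remap, and is broadcast through ProgressChanged.
; The construction script applies colors, icon and initial position; laser focus raises the mesh's material intensity.
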(event `self.ReceiveBeginPlay`
  (bind _bpc_laserinteract (`self.BPC_LaserInteract`))
  (add `/Game/Core/Blueprints/UI/LaserInteractionComponent.IndexAction` _bpc_laserinteract (delegate `LaserEnable`))
  (add `/Game/Core/Blueprints/UI/LaserInteractionComponent.IndexActionStop` _bpc_laserinteract (delegate `LaserDisable`))
  (add `/Game/Core/Blueprints/UI/LaserInteractionComponent.UpdateLocation` _bpc_laserinteract (delegate `UpdateFromLaser`))
  (add `/Game/Core/Blueprints/UI/LaserInteractionComponent.FocusGain` _bpc_laserinteract (delegate `LaserFocusGain`))
  (add `/Game/Core/Blueprints/UI/LaserInteractionComponent.FocusLost` _bpc_laserinteract (delegate `LaserFocusLosr`)))

(event `LaserEnable`
  (params (instigator :type "/Game/Core/Blueprints/Hand/BP_Hand Object Reference"))
  (set `self.LaserActive` true))

(event `LaserDisable`
  (params (instigator :type "/Game/Core/Blueprints/Hand/BP_Hand Object Reference"))
  (set `self.LaserActive` false))

(event `UpdateFromLaser`
  (params (HitLocationLS :type "Vector Structure"))
  (if (`self.LaserActive`)
    (`self.UpdateFromLocation` HitLocationLS)))

(event `LaserFocusGain`
  (`MeshComponent.SetScalarParameterValueOnMaterials` (`self.StaticMesh`) "Intensity" 0.65))

(event `LaserFocusLosr`
  (`MeshComponent.SetScalarParameterValueOnMaterials` (`self.StaticMesh`) "Intensity" 0.0))

(event `self.ReceiveActorBeginOverlap`
  (params (OtherActor :type "Actor Object Reference"))
  (bind _asbp_finger_collider (cast `/Game/Core/Blueprints/Hand/BP_FingerCollider` OtherActor))
  (set `self.Collider` _asbp_finger_collider))

(event `self.ReceiveActorEndOverlap`
  (params (OtherActor :type "Actor Object Reference"))
  (if (== OtherActor (`self.Collider`))
    (set `self.Collider` null)))

(event `self.ReceiveTick`
  (params (DeltaSeconds :type "Float (single-precision)"))
  (bind _collider (`self.Collider`))
  (`/Engine/EditorBlueprintResources/StandardMacros.IsValid` _collider
    (:`Is Valid`
      (`self.UpdateFromLocation` (`KismetMathLibrary.InverseTransformLocation` (`SceneComponent.K2_GetComponentToWorld` (`self.Slider`)) (`SceneComponent.K2_GetComponentLocation` (`/Game/Core/Blueprints/Hand/BP_FingerCollider.Sphere` _collider)))))))

(fn `SetProgress`
  (params (Progress :type "Float (double-precision)"))
  (bind _output_get (set `self.Progress` Progress))
  (`MeshComponent.SetScalarParameterValueOnMaterials` (`self.Slider`) "Progress" _output_get))

(fn `SetSliderPos`
  (`MeshComponent.SetScalarParameterValueOnMaterials` (`self.Slider`) "Progress" (+ (* (`self.Progress`) 0.8) 0.1))
  (`SceneComponent.K2_SetRelativeLocation` (`self.BUtton`) (`KismetMathLibrary.MakeVector` (`KismetMathLibrary.FClamp` (* (- (`self.Progress`) 0.5) 75.0) -37.5 37.5)) false false))

(fn `UpdateFromLocation`
  (params (Location :type "Vector Structure"))
  (bind _output_get (set `self.Progress` (`KismetMathLibrary.FClamp` (+ (/ (.x Location) 75.0) 0.5))))
  (`self.SetSliderPos`)
  (`self.ProgressChanged` _output_get))

(fn `UserConstructionScript`
  (bind _slider (`self.Slider`))
  (`MeshComponent.SetVectorParameterValueOnMaterials` _slider "ActiveColor" (`KismetMathLibrary.Conv_LinearColorToVector` (`self.SliderActive`)))
  (`MeshComponent.SetVectorParameterValueOnMaterials` _slider "InactiveColor" (`KismetMathLibrary.Conv_LinearColorToVector` (`self.SliderInactive`)))
  (`MeshComponent.SetScalarParameterValueOnMaterials` _slider "Progress" (`self.Progress`))
  (bind _returnvalue (`KismetMaterialLibrary.CreateDynamicMaterialInstance` "/Game/Core/Blueprints/Interactive/Buttons/M_ButtonFront.M_ButtonFront"))
  (`PrimitiveComponent.SetMaterial` (`self.BUtton`) 0 _returnvalue)
  (`MaterialInstanceDynamic.SetTextureParameterValue` _returnvalue "Icon" "/Game/Core/Blueprints/Interactive/Buttons/T_SliderDecal.T_SliderDecal")
  (`MaterialInstanceDynamic.SetVectorParameterValue` _returnvalue "Color" (`self.SliderColor`))
  (`self.SetSliderPos`)
  (`MeshComponent.SetVectorParameterValueOnMaterials` (`self.StaticMesh`) "Color" (`KismetMathLibrary.Conv_LinearColorToVector` (`self.OutsideColor`))))