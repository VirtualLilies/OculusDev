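; BP_AmmoMagBase is a base Blueprint for a grabbable ammo magazine that tracks how many rounds it holds.
; On BeginPlay it sets a fixed grab on its GrabbableComponent, with a hand animation and identical left and right transforms on the magazine mesh.
; AddOrRemoveBullets routes through SetNumBullets, which clamps Rounds between zero and MaxRounds.
; AdjustBulletVisibility is an empty function that nothing in this Blueprint calls.
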(event `self.ReceiveBeginPlay`
  (bind _returnvalue (`KismetMathLibrary.MakeTransform` (1.253 -0.92635 7.208684) (struct :`Pitch` -76.309868 :`Yaw` -85.96151 :`Roll` 194.118744)))
  (`/Game/Core/Blueprints/Hand/GrabbableComponent.SetFixedGrab` (`self.GrabbableComponent`) (`self.AmmoMagMesh`) _returnvalue "/Game/Core/Blueprints/Hand/Model/Animations/Grabs/hand_lighter.hand_lighter" _returnvalue))

(fn `AddOrRemoveBullets`
  (params (AddAmmoAmount :type Integer))
  (`self.SetNumBullets` (+ AddAmmoAmount (`self.Rounds`))) ; Call to ensure clamping and everything else is consistent
)

(fn `AdjustBulletVisibility`)

(fn `GetNumBullets`
  (returns (Rounds :type Integer))
  (return (`self.Rounds`)))

(fn `SetNumBullets`
  (params (InValue :type Integer))
  (set `self.Rounds` (`KismetMathLibrary.Clamp` InValue 0 (`self.MaxRounds`))))

(fn `UserConstructionScript`)