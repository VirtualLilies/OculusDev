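; In-world interactive keyboard actor that builds a numpad or keypad layout from 3D buttons and collects the text entered on them.
; On BeginPlay it sizes its plane by type, then spawns and attaches a BP_3DButton for each matching DT_KeyboardKeys row.
; Each button is bound to a type, backspace, clear or enter handler, which edits the optionally displayed text or fires the TextUpdated and EnterKey calls.
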(event `self.ReceiveDestroyed`
  (for _array_element (`self.Buttons`)
    (`self.K2_DestroyActor` _array_element)))

(event `self.ReceiveBeginPlay`
  (`SceneComponent.K2_SetRelativeTransform` (`self.Plane`) (select `/Game/Core/Blueprints/Interactive/Keyboard/EKeyboardType` (`self.Type`) :`NewEnumerator0` (`KismetMathLibrary.MakeTransform` (0.0 -15.0 -30.0) (struct :`Pitch` -90.0 :`Yaw` 180.0 :`Roll` 180.0) (0.5 0.8 0.7)) :`NewEnumerator1` (`KismetMathLibrary.MakeTransform` (0.0 -3.0 -44.0) (struct :`Pitch` -90.0) (0.82 1.85 0.7))) false false)
  (bind _outrownames (`DataTableFunctionLibrary.GetDataTableRowNames` "/Game/Core/Blueprints/Interactive/Keyboard/DT_KeyboardKeys.DT_KeyboardKeys"))
  (for _array_element _outrownames
    (bind _returnvalue (`|GetDataTableRow` "/Game/Core/Blueprints/Interactive/Keyboard/DT_KeyboardKeys.DT_KeyboardKeys" _array_element)
      (:`then`
        (bind (_displaytext _value _position _buttontype _function _keyboardname) (break `/Game/Core/Blueprints/Interactive/Keyboard/KeyboardKeyStruct` _returnvalue))
        (if (`|EnumEquality` (`self.Type`) _keyboardname)
          (bind _returnvalue_2 (`|SpawnActorFromClass` "/Game/Core/Blueprints/Interactive/Buttons/BP_3DButton.BP_3DButton_C" (`KismetMathLibrary.MakeTransform` (0.0 0.0 0.0)) "Undefined" "OverrideRootScale" null (struct :`R` 0.75 :`G` 0.9 :`B` 1.0) null _buttontype (`KismetTextLibrary.Conv_NameToText` _displaytext) (struct :`R` 0.811765 :`G` 0.6) (`KismetStringLibrary.Conv_StringToName` _value) null))
          (bind _output_get (set `self.Button` _returnvalue_2))
          (`KismetArrayLibrary.Array_Add` (`self.Buttons`) _output_get)
          (`self.K2_AttachToActor` _output_get self "None" "SnapToTarget" "SnapToTarget" "SnapToTarget" true)
          (`self.K2_SetActorRelativeLocation` _output_get _position false false)
          (switch `/Game/Core/Blueprints/Interactive/Keyboard/EKeyFunction` _function
            (:`NewEnumerator0`
              (add `/Game/Core/Blueprints/Interactive/Buttons/BP_3DButton.Trigger` (`self.Button`) (delegate `TypeKeyPressed`)))
            (:`NewEnumerator1`
              (add `/Game/Core/Blueprints/Interactive/Buttons/BP_3DButton.Trigger` (`self.Button`) (delegate `BackspaceKeyPressed`)))
            (:`NewEnumerator2`
              (add `/Game/Core/Blueprints/Interactive/Buttons/BP_3DButton.Trigger` (`self.Button`) (delegate `ClearKeyPressed`)))
            (:`NewEnumerator3`
              (add `/Game/Core/Blueprints/Interactive/Buttons/BP_3DButton.Trigger` (`self.Button`) (delegate `EnterKeyPressed`)))))))))

(event `TypeKeyPressed`
  (params (Value :type Name))
  (set `self.Text` (`KismetStringLibrary.Concat_StrStr` (`self.Text`) (`KismetStringLibrary.Conv_NameToString` Value)))
  (`self.UpdateText` :!label _label)
  (`self.TextUpdated` (`self.Text`)))

(event `BackspaceKeyPressed`
  (params (Value :type Name))
  (bind _text (`self.Text`))
  (set `self.Text` (`KismetStringLibrary.GetSubstring` _text 0 (- (`KismetStringLibrary.Len` _text) 1)))
  (goto _label))

(event `ClearKeyPressed`
  (params (Value :type Name))
  (set `self.Text` "")
  (goto _label))

(event `EnterKeyPressed`
  (params (Value :type Name))
  (`self.EnterKey` (`self.Text`)))

(fn `UpdateText`
  (`TextRenderComponent.K2_SetText` (`self.DisplayText`) (`KismetTextLibrary.Conv_StringToText` (`self.Text`))))

(fn `UserConstructionScript`
  (`SceneComponent.SetVisibility` (`self.DisplayText`) (`self.TextVisible`) false))