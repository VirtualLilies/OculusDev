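; BP_PhysicsSkeletal is a skeletal mesh physics object that motion controllers can pick up and drop.
; Pickup releases any current holder, stores the new controller and physics handle, then grabs the named bone at the controller's world location and rotation.
; Drop releases the handle and clears both references.
; IsHeldByMe is a stub that always returns false, and no handle target update occurs in this graph.
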(event `/Game/Core/Blueprints/Interfaces/BPI_Pickup.Pickup`
  (params (MotionController :type "SceneComponent Object Reference") (PhysicsHandle :type "PhysicsHandleComponent Object Reference") (BaneName :type Name))
  (bind (_returnvalue_location _returnvalue_rotation) (`KismetMathLibrary.BreakTransform` (`SceneComponent.K2_GetComponentToWorld` (`self.HoldingMotionController`))))
  (`|ExecutionSequence`
    (:`then_0`
      (`/Engine/EditorBlueprintResources/StandardMacros.IsValid` (`self.HoldingMotionController`)
        (:`Is Valid`
          (`/Game/Core/Blueprints/Interfaces/BPI_Pickup.Drop`))))
    (:`then_1`
      (set `self.HoldingMotionController` MotionController)
      (set `self.HoldingPhysicsHandle` PhysicsHandle))
    (:`then_2`
      (`PhysicsHandleComponent.GrabComponentAtLocationWithRotation` (`self.HoldingPhysicsHandle`) (`self.SkeletalMeshComponent`) BaneName _returnvalue_location _returnvalue_rotation))))

(event `/Game/Core/Blueprints/Interfaces/BPI_Pickup.Drop`
  (`PhysicsHandleComponent.ReleaseComponent` (`self.HoldingPhysicsHandle`))
  (set `self.HoldingMotionController` null)
  (set `self.HoldingPhysicsHandle` null))

(fn `IsHeldByMe`
  (params (MotionController :type "SceneComponent Object Reference"))
  (returns (bIsHeld :type Boolean))
  (return false))

(fn `UserConstructionScript`)