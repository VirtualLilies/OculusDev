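; Base VR pawn that gives the player two motion-controller hands for grabbing and releasing actors.
; On BeginPlay it sets a floor-level tracking origin, then spawns the left and right controller actors, owned by the pawn and snapped to VRRoot.
; Each hand's trigger calls GrabActor on press and ReleaseActor on release, leaving the grab logic to the controller actors.
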(event `self.ReceiveBeginPlay`
  (bind _returnvalue (`KismetMathLibrary.MakeTransform` (0.0 0.0 0.0)))
  ;[1 0 0] BeginPlay()
  ;[0 0 1] VR Settings
  (`HeadMountedDisplayFunctionLibrary.SetTrackingOrigin` "Floor")
  ;[0 1 0] Spawn and attach hands
  (`|ExecutionSequence`
    (:`then_0`
      (bind _returnvalue_2 (`|SpawnActorFromClass` null _returnvalue "AlwaysSpawn" "OverrideRootScale" self "Left" "NewEnumerator0" null)) ; "Hand" is available by checking "Expose on Spawn in the variable on BP_MotionController.
      (bind _output_get (set `self.LeftController` _returnvalue_2))
      (`self.K2_AttachToComponent` _output_get (`self.VRRoot`) "None" "SnapToTarget" "SnapToTarget" "KeepWorld" false))
    (:`then_1`
      (bind _returnvalue_3 (`|SpawnActorFromClass` null _returnvalue "AlwaysSpawn" "OverrideRootScale" self "Right" "NewEnumerator0" null)) ; "Hand" is available by checking "Expose on Spawn in the variable on BP_MotionController.
      (bind _output_get_2 (set `self.RightController` _returnvalue_3))
      (`self.K2_AttachToComponent` _output_get_2 (`self.VRRoot`) "None" "SnapToTarget" "SnapToTarget" "KeepWorld" false))))

(event `Key|MotionController_Right_Trigger`
  (params (Key :type "Key Structure"))
  (bind _rightcontroller (`self.RightController`))
  ;[0 0 1] Grab Inputs
  (:`Pressed`
    (`self.GrabActor` _rightcontroller))
  (:`Released`
    (`self.ReleaseActor` _rightcontroller)))

(event `Key|MotionController_Left_Trigger`
  (params (Key :type "Key Structure"))
  (bind _leftcontroller (`self.LeftController`))
  ;[0 0 1] Grab Inputs
  (:`Pressed`
    (`self.GrabActor` _leftcontroller))
  (:`Released`
    (`self.ReleaseActor` _leftcontroller)))

(fn `UserConstructionScript`)