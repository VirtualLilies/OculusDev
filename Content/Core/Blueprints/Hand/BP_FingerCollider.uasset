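; BP_FingerCollider is a fingertip collider for hand interaction with actors and widgets.
; ActionStart records actors overlapping DetectionSphere that have a FingerActionProxyComponent and forwards the start to that component.
; ActionEnd forwards the end to every recorded actor's proxy, without clearing the list.
; Separately, Sphere overlaps with a WidgetComponent fire the WidgetOverlap dispatcher.
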(event `self.Sphere.OnComponentBeginOverlap`
  (params (OverlappedComponent :type "PrimitiveComponent Object Reference") (OtherActor :type "Actor Object Reference") (OtherComp :type "PrimitiveComponent Object Reference") (OtherBodyIndex :type Integer) (bFromSweep :type Boolean) (SweepResult :type "HitResult Structure (by ref)"))
  (cast `WidgetComponent` OtherComp)
  (`self.WidgetOverlap` false))

(fn `ActionEnd`
  (for _array_element (`self.ActiveActors`)
    (bind _returnvalue (`self.GetComponentByClass` _array_element "/Game/Core/Blueprints/Hand/FingerActionProxyComponent.FingerActionProxyComponent_C"))
    (`/Engine/EditorBlueprintResources/StandardMacros.IsValid` _returnvalue
      (:`Is Valid`
        (`/Game/Core/Blueprints/Hand/FingerActionProxyComponent.ActionEnd` _returnvalue self)))))

(fn `ActionStart`
  (for _array_element (`PrimitiveComponent.GetOverlappingActors` (`self.DetectionSphere`) "/Script/Engine.Actor")
    (bind _returnvalue (`self.GetComponentByClass` _array_element "/Game/Core/Blueprints/Hand/FingerActionProxyComponent.FingerActionProxyComponent_C"))
    (`/Engine/EditorBlueprintResources/StandardMacros.IsValid` _returnvalue
      (:`Is Valid`
        (`KismetArrayLibrary.Array_Add` (`self.ActiveActors`) _array_element)
        (`/Game/Core/Blueprints/Hand/FingerActionProxyComponent.ActionStart` _returnvalue self)))))

(fn `UserConstructionScript`)