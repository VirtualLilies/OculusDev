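; Teleport marker actor that shows a highlightable destination indicator and starts hidden on BeginPlay.
; Activate and deactivate functions toggle the Marker component's visibility.
; When FacingAway is set, activation rotates the actor 180 degrees if the player pawn's location, transformed as a direction (ignoring translation) into local space, has positive X.
; Focus gain and loss functions raise or restore the material's Intensity parameter.
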(event `self.ReceiveBeginPlay`
  (`self.DeactivateMarker`))

(fn `ActivateMarker`
  (`SceneComponent.SetVisibility` (`self.Marker`) true false)
  (if (`self.FacingAway`)
    (if (> (.x (`KismetMathLibrary.TransformDirection` (`KismetMathLibrary.InvertTransform` (`self.GetTransform`)) (`self.K2_GetActorLocation` (`GameplayStatics.GetPlayerPawn` 0)))) 0.0)
      (`self.K2_AddActorWorldRotation` (struct :`Yaw` 180.0)))))

(fn `DeactivateMarker`
  (`SceneComponent.SetVisibility` (`self.Marker`) false false))

(fn `FocusGainMarker`
  (`MeshComponent.SetScalarParameterValueOnMaterials` (`self.Marker`) "Intensity" 5.0))

(fn `FocusLostMarker`
  (`MeshComponent.SetScalarParameterValueOnMaterials` (`self.Marker`) "Intensity" 1.0))

(fn `UserConstructionScript`)