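; VR touch controller for one hand that translates Oculus Touch and motion controller input into actions on its HandActor.
; Thumbstick drives teleport activation and rotation, grip grabs, trigger handles index actions and laser clicks, and face buttons fire thumb and finger actions.
; Each tick feeds analog axes into finger poses and tracks input focus to activate or deactivate the hand.
; Gamepad Special Right toggles the pawn's laser and menu.
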(event `self.ReceiveTick`
  (params (DeltaSeconds :type "Float (single-precision)"))
  (bind _returnvalue (`OculusFunctionLibrary.HasInputFocus`))
  (bind _handactor (`self.HandActor`))
  (`parent.ReceiveTick` DeltaSeconds)
  (`|ExecutionSequence`
    (:`then_0`
      (`self.UpdateAnimationValues`)
      (`self.UpdateHandAnimations`)
      (`self.UpdateTeleportRotation`))
    (:`then_1`
      (if (!= (`self.InputFocus`) _returnvalue)
        (bind _output_get (set `self.InputFocus` _returnvalue))
        (if _output_get
          (`/Game/Core/Blueprints/Hand/BP_Hand.ActivateHand` _handactor)
          (else
            (`self.SetActorHiddenInGame` true)
            (`/Game/Core/Blueprints/Hand/BP_Hand.DeactivateHand` _handactor)))))))

(event `InputAxisKey|MotionController_Left_Thumbstick_Y` :consume false
  (params (AxisValue :type "Float (single-precision)"))
  (if (and (<= AxisValue -0.6) (not (`/Game/Core/Blueprints/Hand/BP_Hand.IsTeleportActive` (`self.HandActor`))) (`|EnumEquality` (`self.Hand`) "Left"))
    (`/Game/Core/Blueprints/Hand/BP_Hand.ActivateTeleport` (`self.HandActor`))))

(event `InputAxisKey|OculusTouch_Left_Thumbstick` :consume false
  (params (AxisValue :type "Float (single-precision)"))
  (if (and (<= AxisValue 0.2) (`/Game/Core/Blueprints/Hand/BP_Hand.IsTeleportActive` (`self.HandActor`)) (`|EnumEquality` (`self.Hand`) "Left") (< (`KismetMathLibrary.Abs` (`self.GetInputAxisKeyValue`)) 0.3) (< (`KismetMathLibrary.Abs` (`self.GetInputAxisKeyValue`)) 0.3))
    (`/Game/Core/Blueprints/Hand/BP_Hand.DeactivateTeleport` (`self.HandActor`))))

(event `InputAxisKey|MotionController_Right_Thumbstick_Y` :consume false
  (params (AxisValue :type "Float (single-precision)"))
  (if (and (<= AxisValue -0.6) (not (`/Game/Core/Blueprints/Hand/BP_Hand.IsTeleportActive` (`self.HandActor`))) (`|EnumEquality` (`self.Hand`) "Right"))
    (`/Game/Core/Blueprints/Hand/BP_Hand.ActivateTeleport` (`self.HandActor`))))

(event `InputAxisKey|OculusTouch_Right_Thumbstick` :consume false
  (params (AxisValue :type "Float (single-precision)"))
  (if (and (<= AxisValue 0.2) (`/Game/Core/Blueprints/Hand/BP_Hand.IsTeleportActive` (`self.HandActor`)) (`|EnumEquality` (`self.Hand`) "Right") (< (`KismetMathLibrary.Abs` (`self.GetInputAxisKeyValue`)) 0.3) (< (`KismetMathLibrary.Abs` (`self.GetInputAxisKeyValue`)) 0.3))
    (`/Game/Core/Blueprints/Hand/BP_Hand.DeactivateTeleport` (`self.HandActor`))))

(event `self.ReceiveBeginPlay`
  (`self.EnableInput` (`GameplayStatics.GetPlayerController` 0)))

(event `Key|MotionController_Right_Trigger` :consume false
  (params (Key :type "Key Structure"))
  (bind _handactor (`self.HandActor`))
  (bind _returnvalue (`|EnumEquality` (`self.Hand`) "Right"))
  (:`Pressed`
    (if _returnvalue
      (`/Game/Core/Blueprints/Hand/BP_Hand.IndexAction` _handactor :!label _label)
      (if (`/Game/Core/Blueprints/Hand/BP_Hand.IsLaserActive` _handactor)
        (`/Game/Core/Blueprints/Hand/BP_Hand.PointerClick` _handactor true))))
  (:`Released`
    (if _returnvalue
      (`/Game/Core/Blueprints/Hand/BP_Hand.IndexActionEnd` _handactor :!label _label_2))))

(event `Key|MotionController_Left_Trigger` :consume false
  (params (Key :type "Key Structure"))
  (bind _returnvalue (`|EnumEquality` (`self.Hand`) "Left"))
  (:`Pressed`
    (if _returnvalue
      (goto _label)))
  (:`Released`
    (if _returnvalue
      (goto _label_2))))

(event `Key|MotionController_Right_FaceButton1` :consume false
  (params (Key :type "Key Structure"))
  (bind _handactor (`self.HandActor`))
  (bind _returnvalue (`|EnumEquality` (`self.Hand`) "Right"))
  (:`Pressed`
    (if _returnvalue
      (`/Game/Core/Blueprints/Hand/BP_Hand.ThumbAction` _handactor :!label _label_3)
      (`/Game/Core/Blueprints/Hand/BP_Hand.FireFingerActions` _handactor)))
  (:`Released`
    (if _returnvalue
      (`/Game/Core/Blueprints/Hand/BP_Hand.ThumbActionEnd` _handactor :!label _label_4)
      (`/Game/Core/Blueprints/Hand/BP_Hand.StopFingerActions` _handactor))))

(event `Key|MotionController_Right_FaceButton2` :consume false
  (params (Key :type "Key Structure"))
  (bind _handactor (`self.HandActor`))
  (bind _returnvalue (`|EnumEquality` (`self.Hand`) "Right"))
  (:`Pressed`
    (if _returnvalue
      (`/Game/Core/Blueprints/Hand/BP_Hand.ThumbAction` _handactor :!label _label_5)))
  (:`Released`
    (if _returnvalue
      (`/Game/Core/Blueprints/Hand/BP_Hand.ThumbActionEnd` _handactor :!label _label_6))))

(event `Key|MotionController_Left_FaceButton1` :consume false
  (params (Key :type "Key Structure"))
  (bind _returnvalue (`|EnumEquality` (`self.Hand`) "Left"))
  (:`Pressed`
    (if _returnvalue
      (goto _label_3)))
  (:`Released`
    (if _returnvalue
      (goto _label_4))))

(event `Key|MotionController_Left_FaceButton2` :consume false
  (params (Key :type "Key Structure"))
  (bind _returnvalue (`|EnumEquality` (`self.Hand`) "Left"))
  (:`Pressed`
    (if _returnvalue
      (goto _label_5)))
  (:`Released`
    (if _returnvalue
      (goto _label_6))))

(event `Key|MotionController_Right_Grip1` :consume false
  (params (Key :type "Key Structure"))
  (bind _handactor (`self.HandActor`))
  (bind _returnvalue (`|EnumEquality` (`self.Hand`) "Right"))
  (:`Pressed`
    (if _returnvalue
      (`/Game/Core/Blueprints/Hand/BP_Hand.AttemptGrab` _handactor :!label _label_7)))
  (:`Released`
    (if _returnvalue
      (`/Game/Core/Blueprints/Hand/BP_Hand.Release` _handactor :!label _label_8))))

(event `Key|MotionController_Left_Grip1` :consume false
  (params (Key :type "Key Structure"))
  (bind _returnvalue (`|EnumEquality` (`self.Hand`) "Left"))
  (:`Pressed`
    (if _returnvalue
      (goto _label_7)))
  (:`Released`
    (if _returnvalue
      (goto _label_8))))

(event `Key|Gamepad_Special_Right`
  (params (Key :type "Key Structure"))
  (bind _mypawn (`/Game/Core/Blueprints/Hand/BP_Hand.MyPawn` (`self.HandActor`)))
  (:`Pressed`
    (`/Game/Core/Blueprints/Pawns/BP_VRPawn.ToggleLaser` _mypawn)
    (`/Game/Core/Blueprints/Pawns/BP_VRPawn.ToggleMenu` _mypawn)))

(fn `UpdateAnimationValues`
  (switch `EControllerHand` (`self.Hand`)
    (:`Left`
      (set `self.ThumbstickX` (`self.GetInputAxisKeyValue`))
      (set `self.ThumbstickY` (`self.GetInputAxisKeyValue`))
      (set `self.TriggerAxis` (`self.GetInputAxisKeyValue`))
      (set `self.GripAxis` (`self.GetInputAxisKeyValue`)))
    (:`Right`
      (set `self.ThumbstickX` (`self.GetInputAxisKeyValue`))
      (set `self.ThumbstickY` (`self.GetInputAxisKeyValue`))
      (set `self.TriggerAxis` (`self.GetInputAxisKeyValue`))
      (set `self.GripAxis` (`self.GetInputAxisKeyValue`)))))

(fn `UpdateHandAnimations`
  (bind _handactor (`self.HandActor`))
  (bind _returnvalue (* (- 1.0 (`self.GetInputAxisKeyValue`)) 0.75))
  (bind _returnvalue_2 (* (- 1.0 (`self.GetInputAxisKeyValue`)) 0.75))
  (switch `EControllerHand` (`self.Hand`)
    (:`Left`
      (`/Game/Core/Blueprints/Hand/BP_Hand.UpdateHandAnimation` _handactor (`KismetMathLibrary.FClamp` (`self.GetInputAxisKeyValue`) (`KismetMathLibrary.FClamp` _returnvalue_2 0.0 0.5)) (`KismetMathLibrary.FClamp` (`self.GetInputAxisKeyValue`) _returnvalue_2) _returnvalue_2 _returnvalue_2 _returnvalue_2))
    (:`Right`
      (`/Game/Core/Blueprints/Hand/BP_Hand.UpdateHandAnimation` _handactor (`KismetMathLibrary.FClamp` (`self.GetInputAxisKeyValue`) (`KismetMathLibrary.FClamp` _returnvalue 0.0 0.5)) (`KismetMathLibrary.FClamp` (`self.GetInputAxisKeyValue`) _returnvalue) _returnvalue _returnvalue _returnvalue))))

(fn `UpdateTeleportRotation`
  (bind _hand (`self.Hand`))
  (bind _returnvalue (`|EnumEquality` _hand "Right"))
  (if (or (`|EnumEquality` _hand "Left") _returnvalue)
    (`/Game/Core/Blueprints/Hand/BP_Hand.AddTeleportRotation` (`self.HandActor`) (select `bool` _returnvalue :`false` (`KismetMathLibrary.DegAtan2` (`self.GetInputAxisKeyValue`) (* (`self.GetInputAxisKeyValue`) -1.0)) :`true` (`KismetMathLibrary.DegAtan2` (`self.GetInputAxisKeyValue`) (* (`self.GetInputAxisKeyValue`) -1.0))))))

(fn `UserConstructionScript`
  (`parent.UserConstructionScript`))